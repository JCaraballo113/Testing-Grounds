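; AI controller for guard NPCs that runs the GuardBehaviour tree on the GuardData blackboard from BeginPlay.
; AI perception updates store sensed actors lacking the "Enemy" tag under the blackboard's enemy key, and clear the key when sensing fails.
; Each tick sets the controlled character's HasEnemy and Shoot flags according to whether the controller has a valid focus actor, which this graph never sets itself.
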(event OnTargetPerceptionUpdated(AIPerception)
  (params (Actor :type Actor%20Object%20Reference) (Stimulus :type AI%20Stimulus%20Structure))
  (CallFunction|UpdateEnemy Actor Stimulus Actor))

(event EventBeginPlay
  (bind _blackboardcomponent (Class|AIController|UseBlackboard "/Game/Dynamic/Character/AI/GuardData.GuardData"))
  (AI|RunBehaviorTree "/Game/Dynamic/Character/AI/GuardBehaviour.GuardBehaviour")
  (Variables|Default|SetBlackboardComp _blackboardcomponent))

(event EventTick
  (params (DeltaSeconds :type Float%20%28single-precision%29))
  (bind _returnvalue (Class|AIController|GetFocusActor))
  (bind _returnvalue_2 (Utilities|IsValid _returnvalue))
  (bind _ascharacter (Utilities|Casting|CastToCharacter (Pawn|GetControlledPawn)))
  (Variables|/Game/Dynamic/Character/Behaviour/Character.Character_C|SetbHasEnemy _ascharacter _returnvalue_2)
  (Variables|/Game/Dynamic/Character/Behaviour/Character.Character_C|SetbShoot _ascharacter _returnvalue_2))

(fn ConstructionScript)

(fn UpdateEnemy
  (params (InputPin :type Actor%20Object%20Reference) (AIStimulus :type AI%20Stimulus%20Structure%20%28by%20ref%29) (self2 :type Actor%20Object%20Reference))
  (bind _blackboardcomp (Variables|Default|GetBlackboardComp))
  (if (not (Actor|ActorHasTag self2 "Enemy"))
    (if (.bSuccessfullySensed (Utilities|Struct|BreakAIStimulus AIStimulus))
      (AI|Components|Blackboard|SetValueasObject _blackboardcomp (Variables|Default|GetEnemyKey) InputPin)
      (else
        (AI|Components|Blackboard|ClearValue _blackboardcomp (Variables|Default|GetEnemyKey))))))