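; AI controller for a patrolling guard NPC that detects targets and makes the guard shoot.
; On BeginPlay it sets up the GuardData blackboard and runs the GuardBehaviour tree.
; AI perception writes sensed actors lacking the "Enemy" tag to the enemy blackboard key and clears it when sensing fails.
; Each tick it sets the pawn's HasEnemy and Shoot flags from whether the controller has a focus actor.
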(event OnTargetPerceptionUpdated(AIPerception)
  (params (Actor :type Actor%20Object%20Reference) (Stimulus :type AI%20Stimulus%20Structure))
  (bind _blackboardcomp (Variables|Default|GetBlackboardComp))
  (if (not (Actor|ActorHasTag Actor "Enemy"))
    (if (.bSuccessfullySensed (Utilities|Struct|BreakAIStimulus Stimulus))
      (AI|Components|Blackboard|SetValueasObject _blackboardcomp (Variables|Default|GetEnemyKey) Actor)
      (else
        (AI|Components|Blackboard|ClearValue _blackboardcomp (Variables|Default|GetEnemyKey))))))

(event EventBeginPlay
  (bind _blackboardcomponent (Class|AIController|UseBlackboard "/Game/Dynamic/NPC/AI/GuardData.GuardData"))
  (AI|RunBehaviorTree "/Game/Dynamic/NPC/AI/GuardBehaviour.GuardBehaviour")
  (Variables|Default|SetBlackboardComp _blackboardcomponent))

(event EventTick
  (params (DeltaSeconds :type Float%20%28single-precision%29))
  (bind _returnvalue (Class|AIController|GetFocusActor))
  (bind _returnvalue_2 (Utilities|IsValid _returnvalue))
  (bind _aspatrolling_guard (Utilities|Casting|CastToPatrollingGuard (Pawn|GetControlledPawn)))
  (Variables|/Game/Dynamic/NPC/Behaviour/PatrollingGuard.PatrollingGuard_C|SetbHasEnemy _aspatrolling_guard _returnvalue_2)
  (Variables|/Game/Dynamic/NPC/Behaviour/PatrollingGuard.PatrollingGuard_C|SetbShoot _aspatrolling_guard _returnvalue_2))

(fn ConstructionScript)